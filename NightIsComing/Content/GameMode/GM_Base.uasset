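; Base game mode for a tower-building game, handling selection, placement, UI updates and night detection from the sun's pitch.
; BeginPlay finds the sun and camera, spawning fallbacks if missing, and creates the play widget only when both exist.
; Tick either moves the pending building along the placement trace or highlights hovered components through custom depth, with stencil marking selection.
; Traces come from camera forward on gamepad, otherwise from the cursor.
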(event `self.ReceiveTick`
  (params (DeltaSeconds :type "Float (single-precision)"))
  (set `self.IsNight` (> (.pitch (`SceneComponent.K2_GetComponentRotation` (`Light.LightComponent` (`self.Sun`)))) (- 90.0 (* (`self.NightPercent`) 180.0))))
  (if (`self.PlaceMode`)
    (`self.PlaceCheck`)
    (else
      (`self.SelectCheck`))))

(event `self.ReceiveBeginPlay`
  (bind _returnvalue (`KismetMathLibrary.MakeTransform` (0.0 0.0 0.0)))
  (bind _returnvalue_2 (`|SpawnActorFromClass` "/Game/Blueprints/Placeable/BP_Tower.BP_Tower_C" _returnvalue "Undefined" "OverrideRootScale" null null))
  (set `self.Placeable` _returnvalue_2)
  (bind _returnvalue_3 (`GameplayStatics.GetActorOfClass` "/Game/Blueprints/Common/BP_Sun.BP_Sun_C"))
  (`/Engine/EditorBlueprintResources/StandardMacros.IsValid` _returnvalue_3
    (:`Is Valid`
      (set `self.Sun` _returnvalue_3)
      (bind _returnvalue_4 (`GameplayStatics.GetActorOfClass` "/Game/Blueprints/Common/BP_Camera.BP_Camera_C"))
      (`/Engine/EditorBlueprintResources/StandardMacros.IsValid` _returnvalue_4
        (:`Is Valid`
          (set `self.Camera` _returnvalue_4)
          (bind _returnvalue_5 (`|CreateWidget` "/Game/Widgets/W_Play.W_Play_C"))
          (`UserWidget.AddToViewport` _returnvalue_5 0)
          (set `self.PlayUI` _returnvalue_5))
        (:`Is Not Valid`
          (`KismetSystemLibrary.PrintString` "Missing Camera!" true true (struct :`R` 1.0 :`G` 0.01 :`A` 1.0) 10.0)
          (bind _returnvalue_6 (`|SpawnActorFromClass` "/Game/Blueprints/Common/BP_Camera.BP_Camera_C" _returnvalue "Undefined" "OverrideRootScale" null null))
          (set `self.Camera` _returnvalue_6))))
    (:`Is Not Valid`
      (`KismetSystemLibrary.PrintString` "Missing Sun!" true true (struct :`R` 1.0 :`G` 0.01 :`A` 1.0) 10.0)
      (bind _returnvalue_7 (`|SpawnActorFromClass` "/Game/Blueprints/Common/BP_Sun.BP_Sun_C" _returnvalue "Undefined" "OverrideRootScale" null null))
      (set `self.Sun` _returnvalue_7))))

(event `SelectCheck`
  (bind _hit (`self.Hit`))
  (bind (_hitresult _returnvalue) (`PlayerController.GetHitResultUnderCursorByChannel` (`GameplayStatics.GetPlayerControllerFromID` 0) "TraceTypeQuery3" true))
  (bind _camera (`/Game/Blueprints/Common/BP_Camera.Camera` (`self.Camera`)))
  (bind (_bblockinghit _binitialoverlap _time _distance _location _impactpoint _normal _impactnormal _physmat _hitactor _hitcomponent) (`GameplayStatics.BreakHitResult` _hitresult))
  (bind _returnvalue_2 (`SceneComponent.K2_GetComponentLocation` _camera))
  (`/Engine/EditorBlueprintResources/StandardMacros.IsValid` _hit
    (:`Is Valid`
      (`PrimitiveComponent.SetRenderCustomDepth` _hit false)
      (set `self.Hit` null))
    (:`Is Not Valid`
      _))
  (if (`self.Gamepad`)
    (bind (_outhit _returnvalue_3) (`KismetSystemLibrary.LineTraceSingle` _returnvalue_2 (+ (* (`KismetMathLibrary.GreaterGreater_VectorRotator` (`KismetMathLibrary.MakeVector` 1.0) (`SceneComponent.K2_GetComponentRotation` _camera)) 10000.0) _returnvalue_2) "TraceTypeQuery3"))
    (if _returnvalue_3
      (bind (_bblockinghit_2 _binitialoverlap_2 _time_2 _distance_2 _location_2 _impactpoint_2 _normal_2 _impactnormal_2 _physmat_2 _hitactor_2 _hitcomponent_2) (`GameplayStatics.BreakHitResult` _outhit))
      (if (!= (`self.Selection`) _hitcomponent_2)
        (bind _output_get (set `self.Hit` _hitcomponent_2))
        (`PrimitiveComponent.SetRenderCustomDepth` _output_get true)))
    (elif _returnvalue
      (if (!= (`self.Selection`) _hitcomponent)
        (bind _output_get_2 (set `self.Hit` _hitcomponent))
        (`PrimitiveComponent.SetRenderCustomDepth` _output_get_2 true)))))

(event `ToGamepad`
  (set `self.Gamepad` true))

(event `ToKeyboard`
  (set `self.Gamepad` false))

(event `Select`
  (bind _selection (`self.Selection`))
  (bind _hit (`self.Hit`))
  (`/Engine/EditorBlueprintResources/StandardMacros.IsValid` _selection
    (:`Is Valid`
      (`PrimitiveComponent.SetCustomDepthStencilValue` _selection 0)
      (`PrimitiveComponent.SetRenderCustomDepth` _selection false))
    (:`Is Not Valid`
      _))
  (`/Engine/EditorBlueprintResources/StandardMacros.IsValid` _hit
    (:`Is Valid`
      (`PrimitiveComponent.SetCustomDepthStencilValue` _hit 255)
      (set `self.Selection` _hit)
      (set `self.Hit` null))))

(event `Select/Place`
  (if (`self.PlaceMode`)
    (bind _placed (message `/Game/Blueprints/Common/I_Placeable.Place` (`self.Placeable`)))
    (if _placed
      (set `self.Placeable` null)
      (set `self.PlaceMode` false)
      (`/Game/Widgets/W_Play.Place` (`self.PlayUI`)))
    (else
      (`self.Select`))))

(event `PauseTime`
  (set `self.TimePaused` true))

(event `UnpauseTime`
  (set `self.TimePaused` false))

(event `NextTower`
  (`/Game/Widgets/W_Play.NextTower` (`self.PlayUI`)))

(event `PreviousTower`
  (`/Game/Widgets/W_Play.PrevTower` (`self.PlayUI`)))

(event `PlaceCheck`
  (bind _placeable (`self.Placeable`))
  (bind _camera (`/Game/Blueprints/Common/BP_Camera.Camera` (`self.Camera`)))
  (bind _returnvalue (`SceneComponent.K2_GetComponentLocation` _camera))
  (`/Engine/EditorBlueprintResources/StandardMacros.IsValid` _placeable
    (:`Is Valid`
      (bind _offset (message `/Game/Blueprints/Common/I_Placeable.GetOffset` _placeable))
      (if (`self.Gamepad`)
        (bind _outhit (`KismetSystemLibrary.LineTraceSingle` _returnvalue (+ (* (`KismetMathLibrary.GreaterGreater_VectorRotator` (`KismetMathLibrary.MakeVector` 1.0) (`SceneComponent.K2_GetComponentRotation` _camera)) 10000.0) _returnvalue) "TraceTypeQuery4"))
        (`self.K2_SetActorLocation` _placeable (+ (`.Location` (`GameplayStatics.BreakHitResult` _outhit)) _offset) false false)
        (else
          (`self.K2_SetActorLocation` _placeable (+ _offset (`.Location` (`GameplayStatics.BreakHitResult` (`PlayerController.GetHitResultUnderCursorByChannel` (`GameplayStatics.GetPlayerControllerFromID` 0) "TraceTypeQuery4" true)))) false false))))))

(event `SpawnBuilding`
  (params (TowerType :type "/Game/Blueprints/Common/S_TowerTypeW Structure"))
  (bind _returnvalue (`|SpawnActorFromClass` (`.TowerType_3_8F56DABA479BD206D993878A9966F8C9` (break `/Game/Blueprints/Common/S_TowerTypeW` TowerType)) (`KismetMathLibrary.MakeTransform` (`.Location` (`GameplayStatics.BreakHitResult` (`PlayerController.GetHitResultUnderCursorByChannel` (`GameplayStatics.GetPlayerControllerFromID` 0) "TraceTypeQuery4" true)))) "Undefined" "OverrideRootScale" null null))
  (set `self.Placeable` _returnvalue)
  (set `self.PlaceMode` true))

(event `UpdateResources`
  (bind _placeable (`self.Placeable`))
  (`/Game/Widgets/W_Play.UpdateCounts` (`self.PlayUI`))
  (`/Engine/EditorBlueprintResources/StandardMacros.IsValid` _placeable
    (:`Is Valid`
      (message `/Game/Blueprints/Common/I_Placeable.UpdateResources` _placeable))))

(fn `UserConstructionScript`)