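; BP_Tower is a placeable tower that previews whether its current spot is valid before being placed.
; On BeginPlay it applies a dynamic M_Place material to its mesh.
; While placing, actor overlap begin and end events toggle CanPlace and tint the preview red or green, without counting simultaneous overlaps.
; Place swaps to M_Basic and ends placing when allowed, returning CanPlace, and GetOffset supplies a fixed vertical offset.
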(event `self.ReceiveBeginPlay`
  (bind _returnvalue (`PrimitiveComponent.CreateDynamicMaterialInstance` (`self.StaticMeshComponent`) 0 "/Game/Materials/M_Place.M_Place" "None"))
  (set `self.PlaceMaterial` _returnvalue))

(event `self.ReceiveActorBeginOverlap`
  (params (OtherActor :type "Actor Object Reference"))
  (if (`self.Placing`)
    (set `self.CanPlace` false)
    (`MaterialInstanceDynamic.SetVectorParameterValue` (`self.PlaceMaterial`) "Color" (make `LinearColor` 1.0 0.0 0.0 0.5))))

(event `self.ReceiveTick`
  (params (DeltaSeconds :type "Float (single-precision)")))

(event `self.ReceiveActorEndOverlap`
  (params (OtherActor :type "Actor Object Reference"))
  (if (`self.Placing`)
    (set `self.CanPlace` true)
    (`MaterialInstanceDynamic.SetVectorParameterValue` (`self.PlaceMaterial`) "Color" (make `LinearColor` 0.0 0.33 0.0 0.5))))

(fn `GetOffset`
  (returns (Offset :type "Vector Structure"))
  (return (0.0 0.0 50.0)))

(fn `Place`
  (returns (Placed :type Boolean))
  (if (`self.CanPlace`)
    (`PrimitiveComponent.SetMaterial` (`self.StaticMeshComponent`) 0 "/Game/Materials/M_Basic.M_Basic")
    (set `self.Placing` false))
  (return (`self.CanPlace`)))

(fn `UserConstructionScript`)