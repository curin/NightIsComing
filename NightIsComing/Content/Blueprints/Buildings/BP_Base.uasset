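; BP_Base is the base building, which generates gold and lumber during the day and ends the game when its Destroy event fires.
; It sets max health and natural regen on BeginPlay before calling the parent.
; Outside night, Tick adds income to the game manager's Resources array, carrying fractions between frames so totals stay whole, then calls UpdateResources.
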(event `self.ReceiveBeginPlay`
  (set `self.MaxHealth` 200)
  (set `self.NaturalRegen` 1.0)
  (`parent.ReceiveBeginPlay`))

(event `self.ReceiveTick`
  (params (DeltaSeconds :type "Float (single-precision)"))
  (bind _gm (`self.GM`))
  (bind _resources (`/Game/GameMode/GM_Base.Resources` _gm))
  (bind _returnvalue (+ (* DeltaSeconds (`self.GoldSpeed`)) (`self.FractionalGold`)))
  (bind _returnvalue_2 (+ (* DeltaSeconds (`self.LumberSpeed`)) (`self.FractionalLumber`)))
  (`parent.ReceiveTick` DeltaSeconds)
  (if (not (`/Game/GameMode/GM_Base.IsNight` _gm))
    (set `self.FractionalGold` (`KismetMathLibrary.Fraction` _returnvalue))
    (`KismetArrayLibrary.Array_Set` _resources 0 (+ (`|GetArrayItem` _resources) (`KismetMathLibrary.FFloor64` _returnvalue)))
    (set `self.FractionalLumber` (`KismetMathLibrary.Fraction` _returnvalue_2))
    (`KismetArrayLibrary.Array_Set` _resources 1 (+ (`|GetArrayItem` _resources 1) (`KismetMathLibrary.FFloor64` _returnvalue_2)))
    (`/Game/GameMode/GM_Base.UpdateResources` _gm)))

(event `self.Destroy`
  (`/Game/GameMode/GM_Base.GameOver` (`self.GM`)))

(fn `UserConstructionScript`
  (`parent.UserConstructionScript`))