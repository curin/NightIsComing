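; BP_Structure is a building actor with health, natural regeneration, damage handling and a friendly health bar widget.
; Tick adds regeneration to health, carrying the fractional part in FloatingHealth so CurrentHealth stays an integer, then clamps to MaxHealth.
; Damage destroys the actor at zero health after calling an empty Destroy event.
; Tick, Damage and Select refresh the bar, which updates only while the widget is visible.
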(event `self.ReceiveBeginPlay`
  (set `self.CurrentHealth` (`self.MaxHealth`))
  (bind _asgm_base (cast `/Game/GameMode/GM_Base` (`GameplayStatics.GetGameMode`)))
  (set `self.GM` _asgm_base)
  (bind _returnvalue (`|CreateWidget` "/Game/Widgets/W_FriendlyHealth.W_FriendlyHealth_C" (`GameplayStatics.GetPlayerControllerFromID` 0)))
  (bind _output_get (set `self.HealthBar` _returnvalue))
  (`WidgetComponent.SetWidget` (`self.Widget`) _output_get)
  (`/Game/Widgets/W_FriendlyHealth.UpdateHealth` (`self.HealthBar`) 1.0))

(event `self.ReceiveTick`
  (params (DeltaSeconds :type "Float (single-precision)"))
  (bind _maxhealth (`self.MaxHealth`))
  (bind _returnvalue (+ (* DeltaSeconds (`self.NaturalRegen`)) (`self.FloatingHealth`) (`KismetMathLibrary.Conv_IntToDouble` (`self.CurrentHealth`))))
  (set `self.CurrentHealth` (`KismetMathLibrary.FFloor` _returnvalue))
  (set `self.FloatingHealth` (`KismetMathLibrary.Fraction` _returnvalue))
  (if (> (`self.CurrentHealth`) _maxhealth)
    (set `self.CurrentHealth` _maxhealth))
  (`self.UpdateHealthBar`))

(event `/Game/Blueprints/Common/I_Structure.Damage`
  (params (Damage :type Integer))
  (bind _output_get (set `self.CurrentHealth` (- (`self.CurrentHealth`) Damage)))
  (`self.UpdateHealthBar`)
  (if (<= _output_get 0)
    (`self.Destroy`)
    (`self.K2_DestroyActor`)))

(event `Destroy`)

(event `UpdateHealthBar`
  (if (`SceneComponent.IsVisible` (`self.Widget`))
    (`/Game/Widgets/W_FriendlyHealth.UpdateHealth` (`self.HealthBar`) (/ (`KismetMathLibrary.Conv_IntToDouble` (`self.CurrentHealth`)) (`KismetMathLibrary.Conv_IntToDouble` (`self.MaxHealth`))))))

(event `/Game/Blueprints/Common/I_Structure.Select`
  (`self.UpdateHealthBar`))

(fn `UserConstructionScript`)