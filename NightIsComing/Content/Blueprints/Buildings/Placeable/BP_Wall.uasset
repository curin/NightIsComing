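; Placeable wall building that previews its placement, spends resources when placed and offers range helpers for finding enemies.
; While placing, overlaps and unaffordable costs share a blocker count that sets CanPlace and tints the preview material red or green.
; Place swaps to the final material, deducts costs through GM and calls the empty OnPlace hook.
; Selection shows the health bar and a range ring scaled from Range, while enemy checks use squared XY distance.
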(event `self.ReceiveBeginPlay`
  (bind _range (`self.Range`))
  (bind _rangering (`self.RangeRing`))
  (bind _returnvalue (/ (* _range 2.0) 256.0))
  (`parent.ReceiveBeginPlay`)
  (bind _returnvalue_2 (`PrimitiveComponent.CreateDynamicMaterialInstance` (`self.StaticMeshComponent`) 0 "/Game/Materials/M_Place.M_Place" "None"))
  (set `self.PlaceMaterial` _returnvalue_2)
  (`/Game/Blueprints/Common/I_Placeable.UpdateResources`)
  (`Widget.SetVisibility` (`self.HealthBar`) "Hidden")
  (set `self.RangeSquared` (`KismetMathLibrary.Square` _range))
  (if (> (`self.Range`) 0.0)
    (`SceneComponent.SetWorldScale3D` _rangering (`KismetMathLibrary.MakeVector` _returnvalue _returnvalue _returnvalue))
    (else
      (`SceneComponent.SetVisibility` _rangering false false))))

(event `self.ReceiveActorBeginOverlap`
  (params (OtherActor :type "Actor Object Reference"))
  (`parent.ReceiveActorBeginOverlap` OtherActor)
  (if (`self.Placing`)
    (`self.AddToCount`)))

(event `self.ReceiveActorEndOverlap`
  (params (OtherActor :type "Actor Object Reference"))
  (if (`self.Placing`)
    (`self.RemoveFromCount`)))

(event `RemoveFromCount`
  (bind _result (`/Engine/EditorBlueprintResources/StandardMacros.DecrementInt` (`self.Count`))
    (:`  `
      (if (== _result 0)
        (set `self.CanPlace` true)
        (`MaterialInstanceDynamic.SetVectorParameterValue` (`self.PlaceMaterial`) "Color" (make `LinearColor` 0.0 0.33 0.0 0.5))))))

(event `AddToCount`
  (set `self.CanPlace` false)
  (`MaterialInstanceDynamic.SetVectorParameterValue` (`self.PlaceMaterial`) "Color" (make `LinearColor` 1.0 0.0 0.0 0.5))
  (`/Engine/EditorBlueprintResources/StandardMacros.IncrementInt` (`self.Count`)))

(event `/Game/Blueprints/Common/I_Placeable.UpdateResources`
  (bind _needresources (`self.NeedResources`))
  (set `self.enough` true)
  (for (_array_element _array_index) (`self.Costs`)
    (if (< (`|GetArrayItem` (`/Game/GameMode/GM_Base.Resources` (`self.GM`)) _array_index) _array_element)
      (set `self.enough` false)
      (break)))
  (if (`self.enough`)
    (if _needresources
      (set `self.NeedResources` false)
      (`self.RemoveFromCount`))
    (elif (not _needresources)
      (set `self.NeedResources` true)
      (`self.AddToCount`))))

(event `/Game/Blueprints/Common/I_Structure.Select`
  (`Widget.SetVisibility` (`self.HealthBar`) "Visible")
  (`SceneComponent.SetVisibility` (`self.RangeRing`) (> (`self.Range`) 0.0) false))

(event `/Game/Blueprints/Common/I_Structure.Deselect`
  (`Widget.SetVisibility` (`self.HealthBar`) "Hidden")
  (`SceneComponent.SetVisibility` (`self.RangeRing`) false false))

(event `OnPlace`)

(fn `CheckRange`
  (params (Target :type "Actor Object Reference"))
  (returns (InRange :type Boolean))
  (return (<= (`KismetMathLibrary.VSizeXYSquared` (- (`self.K2_GetActorLocation`) (`self.K2_GetActorLocation` Target))) (`self.RangeSquared`))))

(fn `FindInRangeEnemy`
  (returns (NearestEnemy :type "Actor Object Reference") (EnemyInRange :type Boolean))
  (locals (Dist :type "Float (double-precision)") (Nearest :type Integer))
  (set `local.Dist` 1.2919594778391216e+19)
  (set `local.Nearest` -1)
  (bind _outactors (`GameplayStatics.GetAllActorsWithInterface` "/Game/Blueprints/Common/I_Enemy.I_Enemy_C"))
  (if (== (`KismetArrayLibrary.Array_Length` _outactors) 0)
    (return null false)
    (else
      (for (_array_element _array_index) _outactors
        (bind _returnvalue (`KismetMathLibrary.VSizeXYSquared` (- (`self.K2_GetActorLocation`) (`self.K2_GetActorLocation` _array_element))))
        (if (< _returnvalue (`local.Dist`))
          (set `local.Nearest` _array_index)
          (set `local.Dist` _returnvalue)))
      (if (<= (`local.Dist`) (`self.RangeSquared`))
        (return (`|GetArrayItem` _outactors (`local.Nearest`)) true)
        (else
          (return null false))))))

(fn `GetOffset`
  (returns (Offset :type "Vector Structure"))
  (return (0.0 0.0 50.0)))

(fn `Place`
  (returns (Placed :type Boolean))
  (bind _gm (`self.GM`))
  (bind _resources (`/Game/GameMode/GM_Base.Resources` _gm))
  (if (`self.CanPlace`)
    (bind _returnvalue (`PrimitiveComponent.CreateDynamicMaterialInstance` (`self.StaticMeshComponent`) 0 "/Game/Materials/M_Basic.M_Basic" "None"))
    (bind _output_get (set `self.PlacedMaterial` _returnvalue))
    (`PrimitiveComponent.SetMaterial` (`self.StaticMeshComponent`) 0 _output_get)
    (set `self.Placing` false)
    (set `/Game/GameMode/GM_Base.Placeable` null _gm)
    (for (_array_element _array_index) (`self.Costs`)
      (`KismetArrayLibrary.Array_Set` _resources _array_index (- (`|GetArrayItem` _resources _array_index) _array_element)))
    (`/Game/GameMode/GM_Base.UpdateResources` _gm)
    (`MaterialInstanceDynamic.SetVectorParameterValue` (`self.PlacedMaterial`) "Color" (`self.Color`))
    (`SceneComponent.SetVisibility` (`self.RangeRing`) false false)
    (`self.OnPlace`))
  (return (`self.CanPlace`)))

(fn `UserConstructionScript`
  (`parent.UserConstructionScript`))