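; Placeable tower building that automatically finds and damages enemies once it is placed.
; OnPlace starts a delayed Search loop that calls FindInRangeEnemy and stores the nearest enemy as Target.
; Attack then sends DamageMessage to the Target on a cooldown until it becomes invalid, then returns to Search.
; Both states are self-calling events with Delays rather than Tick, and range is not rechecked during attacks.
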(event `self.ReceiveBeginPlay`
  (`parent.ReceiveBeginPlay`))

(event `self.OnPlace`
  (`self.Search`))

(event `Search`
  (`KismetSystemLibrary.Delay` (`self.SearchCooldown`))
  (bind (_nearestenemy _enemyinrange) (`self.FindInRangeEnemy`))
  (if _enemyinrange
    (set `self.Target` _nearestenemy)
    (`self.Attack`)
    (else
      (`self.Search`))))

(event `Attack`
  (bind _target (`self.Target`))
  (`/Engine/EditorBlueprintResources/StandardMacros.IsValid` _target
    (:`Is Valid`
      (message `/Game/Blueprints/Common/I_Enemy.Damage` _target (`self.DMG`))
      (`KismetSystemLibrary.Delay` (`self.AttackCooldown`))
      (`self.Attack`))
    (:`Is Not Valid`
      (`self.Search`))))

(fn `UserConstructionScript`
  (`parent.UserConstructionScript`))