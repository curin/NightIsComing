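; BP_ResourceBuilding is a placeable building that passively produces resources while it is placed and it is not night.
; Each Tick scales every ResourceGenerationRate entry by delta time and adds the stored ResourceFraction.
; Whole units are added to the matching index of GM.Resources, while the fractional remainder carries over to later frames.
; After the loop it calls GM.UpdateResources, so this runs every producing frame.
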(event `self.ReceiveTick`
  (params (DeltaSeconds :type "Float (single-precision)"))
  (bind _gm (`self.GM`))
  (bind _resourcefraction (`self.ResourceFraction`))
  (bind _resources (`/Game/GameMode/GM_Base.Resources` _gm))
  (`parent.ReceiveTick` DeltaSeconds)
  (if (and (not (`self.Placing`)) (not (`/Game/GameMode/GM_Base.IsNight` (`self.GM`))))
    (for (_array_element _array_index) (`self.ResourceGenerationRate`)
      (bind _returnvalue (+ (* _array_element DeltaSeconds) (`|GetArrayItem` _resourcefraction _array_index)))
      (`KismetArrayLibrary.Array_Set` _resourcefraction _array_index (`KismetMathLibrary.Fraction` _returnvalue))
      (`KismetArrayLibrary.Array_Set` _resources _array_index (+ (`KismetMathLibrary.FFloor64` _returnvalue) (`|GetArrayItem` _resources _array_index))))
    (`/Game/GameMode/GM_Base.UpdateResources` _gm)))

(fn `UserConstructionScript`
  (`parent.UserConstructionScript`))