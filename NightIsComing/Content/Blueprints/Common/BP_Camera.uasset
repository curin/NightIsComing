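; BP_Camera is an orbit camera that the player pans, rotates and zooms around a movable focus point.
; Each tick places the camera on a sphere from distance and two angles, aimed at the root; holding CameraControl rotates it with clamped pitch.
; Move axes slide the root relative to camera yaw, and zoom clamps the distance.
; Select and keyboard/gamepad switch inputs are forwarded to the GM_Base game mode.
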(event `self.ReceiveBeginPlay`
  (bind _asgm_base (cast `/Game/GameMode/GM_Base` (`GameplayStatics.GetGameMode`)))
  (set `self.GM` _asgm_base))

(event `self.ReceiveTick`
  (params (DeltaSeconds :type "Float (single-precision)"))
  (bind _rotvert (`self.RotVert`))
  (bind _rothor (`self.RotHor`))
  (bind _dist (`self.Dist`))
  (bind _returnvalue (`KismetMathLibrary.DegCos` _rotvert))
  (bind _returnvalue_2 (`KismetMathLibrary.MakeVector` (* _dist (* (`KismetMathLibrary.DegCos` _rothor) _returnvalue)) (* _dist (* (`KismetMathLibrary.DegSin` _rothor) _returnvalue)) (* _dist (`KismetMathLibrary.DegSin` _rotvert))))
  (`SceneComponent.K2_SetRelativeLocationAndRotation` (`self.Camera`) _returnvalue_2 (`KismetMathLibrary.FindLookAtRotation` _returnvalue_2 (`KismetMathLibrary.MakeVector` 0.0)) false false)
  (if (`self.CameraControl`)
    (set `self.RotHor` (+ (* (`self.GetInputAxisValue`) (`self.RotationSpeed`)) (`self.RotHor`)))
    (set `self.RotVert` (`KismetMathLibrary.ClampAngle` (+ (`self.RotVert`) (* (`self.GetInputAxisValue`) (`self.RotationSpeed`))) 5.0 85.0))))

(event `InputAction|CameraControl`
  (params (Key :type "Key Structure"))
  (:`Pressed`
    (set `self.CameraControl` true))
  (:`Released`
    (set `self.CameraControl` false)))

(event `InputAxis|MoveUp`
  (params (AxisValue :type "Float (single-precision)"))
  (`SceneComponent.K2_AddWorldOffset` (`self.DefaultSceneRoot`) (`KismetMathLibrary.GreaterGreater_VectorRotator` (* (`KismetMathLibrary.MakeVector` AxisValue) (`self.Speed`)) (`KismetMathLibrary.MakeRotator` 0.0 0.0 (.yaw (`SceneComponent.K2_GetComponentRotation` (`self.Camera`))))) false false))

(event `InputAxis|MoveRight`
  (params (AxisValue :type "Float (single-precision)"))
  (`SceneComponent.K2_AddWorldOffset` (`self.DefaultSceneRoot`) (`KismetMathLibrary.GreaterGreater_VectorRotator` (* (`KismetMathLibrary.MakeVector` 0.0 AxisValue) (`self.Speed`)) (`KismetMathLibrary.MakeRotator` 0.0 0.0 (.yaw (`SceneComponent.K2_GetComponentRotation` (`self.Camera`))))) false false))

(event `InputAxis|CameraZoom`
  (params (AxisValue :type "Float (single-precision)"))
  (set `self.Dist` (`KismetMathLibrary.FClamp` (+ (* AxisValue (`self.ZoomSpeed`) -1.0) (`self.Dist`)) (`self.MinZoom`) (`self.MaxZoom`))))

(event `InputAction|ControllerSwitch`
  (params (Key :type "Key Structure"))
  (:`Pressed`
    (`/Game/GameMode/GM_Base.ToGamepad` (`self.GM`))))

(event `InputAction|KeyboardSwitch`
  (params (Key :type "Key Structure"))
  (:`Pressed`
    (`/Game/GameMode/GM_Base.ToKeyboard` (`self.GM`))))

(event `InputAction|Select`
  (params (Key :type "Key Structure"))
  (:`Pressed`
    (`/Game/GameMode/GM_Base.Select` (`self.GM`))))

(fn `UserConstructionScript`)