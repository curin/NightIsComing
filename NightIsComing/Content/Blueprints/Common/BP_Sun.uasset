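; BP_Sun drives a day cycle by rotating itself around its local pitch axis at one full turn per DayLength seconds.
; It caches the GM_Base game mode on BeginPlay and halts the rotation while that game mode's TimePaused is set.
; Each tick it also calls UpdateSunDirection on the Sky reference, even while time is paused.
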(event `self.ReceiveBeginPlay`
  (bind _asgm_base (cast `/Game/GameMode/GM_Base` (`GameplayStatics.GetGameMode`)))
  (set `self.GM` _asgm_base))

(event `self.ReceiveTick`
  (params (DeltaSeconds :type "Float (single-precision)"))
  (if (not (`/Game/GameMode/GM_Base.TimePaused` (`self.GM`)))
    (`self.K2_AddActorLocalRotation` self (`KismetMathLibrary.MakeRotator` 0.0 (* DeltaSeconds (/ 360.0 (`self.DayLength`)))) false false))
  (`/Engine/EngineSky/BP_Sky_Sphere.UpdateSunDirection` (`self.Sky`)))

(fn `UserConstructionScript`)