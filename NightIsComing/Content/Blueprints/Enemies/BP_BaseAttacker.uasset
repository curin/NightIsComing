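; Base enemy that seeks out a base to attack, falling back to the nearest structure when movement fails.
; On BeginPlay it targets the result of FindBase and uses AI MoveTo; a failed move while not attacking retargets through FindNearestStructure.
; Tick compares squared XY distance to RangeSquared, then sets Attacking, calls the empty Attack event and re-finds the base.
; An invalid target also triggers a new base search.
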(event `self.ReceiveBeginPlay`
  (`parent.ReceiveBeginPlay`)
  (bind _base (`self.FindBase`))
  (set `self.Target` _base)
  (`self.MoveToTarget`))

(event `self.ReceiveTick`
  (params (DeltaSeconds :type "Float (single-precision)"))
  (bind _target (`self.Target`))
  (`parent.ReceiveTick` DeltaSeconds)
  (`/Engine/EditorBlueprintResources/StandardMacros.IsValid` _target
    (:`Is Valid`
      (if (< (`KismetMathLibrary.VSizeXYSquared` (- (`SceneComponent.K2_GetComponentLocation` (`self.CapsuleComponent`)) (`self.K2_GetActorLocation` _target))) (`self.RangeSquared`))
        (set `self.Attacking` true)
        (`self.Attack`)
        (`self.FindNewTarget`)))
    (:`Is Not Valid`
      (`self.FindNewTarget`))))

(event `MoveToTarget`
  (`|AIMoveTo` self (0.0 0.0 0.0) (`self.Target`)
    (:`OnFail`
      (if (not (`self.Attacking`))
        (`self.FindAlternateTarget`)))))

(event `Attack`)

(event `FindNewTarget`
  (bind _base (`self.FindBase`))
  (set `self.Target` _base)
  (`self.MoveToTarget`))

(event `FindAlternateTarget`
  (bind _location (`self.FindNearestStructure`))
  (set `self.Target` _location)
  (`self.MoveToTarget`))

(fn `UserConstructionScript`
  (`parent.UserConstructionScript`))