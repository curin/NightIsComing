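; Enemy actor that tracks health, shows a health bar while selected, and provides targeting helpers.
; BeginPlay caches GM_Base and creates a hidden W_EnemyHealth in its widget component, which Select and Deselect show or hide.
; Damage lowers health and refreshes the bar, calling the empty Destroy event before removing the actor at zero.
; FindBase and FindNearestStructure return the closest BP_Base or I_Structure actor by squared XY distance, but are not called here.
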(event `self.ReceiveBeginPlay`
  (set `self.CurrentHealth` (`self.MaxHealth`))
  (bind _asgm_base (cast `/Game/GameMode/GM_Base` (`GameplayStatics.GetGameMode`)))
  (set `self.GM` _asgm_base)
  (bind _returnvalue (`|CreateWidget` "/Game/Widgets/W_EnemyHealth.W_EnemyHealth_C" (`GameplayStatics.GetPlayerControllerFromID` 0)))
  (bind _output_get (set `self.HealthBar` _returnvalue))
  (`WidgetComponent.SetWidget` (`self.Widget`) _output_get)
  (`/Game/Widgets/W_EnemyHealth.UpdateHealth` _output_get 1.0)
  (`Widget.SetVisibility` (`self.HealthBar`) "Hidden"))

(event `/Game/Blueprints/Common/I_Enemy.Damage`
  (params (Damage :type Integer))
  (bind _output_get (set `self.CurrentHealth` (- (`self.CurrentHealth`) Damage)))
  (`self.UpdateHealthBar`)
  (if (<= _output_get 0)
    (`self.Destroy`)
    (`self.K2_DestroyActor`)))

(event `Destroy`)

(event `UpdateHealthBar`
  (if (`SceneComponent.IsVisible` (`self.Widget`))
    (`/Game/Widgets/W_EnemyHealth.UpdateHealth` (`self.HealthBar`) (/ (`KismetMathLibrary.Conv_IntToDouble` (`self.CurrentHealth`)) (`KismetMathLibrary.Conv_IntToDouble` (`self.MaxHealth`))))))

(event `/Game/Blueprints/Common/I_Enemy.Select`
  (`Widget.SetVisibility` (`self.HealthBar`) "Visible")
  (`self.UpdateHealthBar`))

(event `/Game/Blueprints/Common/I_Enemy.Deselect`
  (`Widget.SetVisibility` (`self.HealthBar`) "Hidden"))

(fn `FindBase`
  (returns (Base :type "Actor Object Reference"))
  (locals (shortest :type Integer :default -1) (dist :type "Float (double-precision)" :default 7.985668304788198e+30))
  (set `local.dist` 9.632337585829315e+18)
  (set `local.shortest` -1)
  (bind _outactors (`GameplayStatics.GetAllActorsOfClass` "/Game/Blueprints/Buildings/BP_Base.BP_Base_C"))
  (for (_array_element _array_index) _outactors
    (bind _returnvalue (`KismetMathLibrary.VSizeXYSquared` (- (`self.K2_GetActorLocation` _array_element) (`SceneComponent.K2_GetComponentLocation` (`self.DefaultSceneRoot`)))))
    (if (< _returnvalue (`local.dist`))
      (set `local.shortest` _array_index)
      (set `local.dist` _returnvalue)))
  (return (`|GetArrayItem` _outactors (`local.shortest`))))

(fn `FindNearestStructure`
  (returns (Location :type "Actor Object Reference"))
  (locals (dist :type "Float (double-precision)") (shortest :type Integer))
  (set `local.dist` 9.632337585829315e+18)
  (set `local.shortest` -1)
  (bind _outactors (`GameplayStatics.GetAllActorsWithInterface` "/Game/Blueprints/Common/I_Structure.I_Structure_C"))
  (for (_array_element _array_index) _outactors
    (bind _returnvalue (`KismetMathLibrary.VSizeXYSquared` (- (`self.K2_GetActorLocation` _array_element) (`SceneComponent.K2_GetComponentLocation` (`self.DefaultSceneRoot`)))))
    (if (< _returnvalue (`local.dist`))
      (set `local.shortest` _array_index)
      (set `local.dist` _returnvalue)))
  (return (`|GetArrayItem` _outactors (`local.shortest`))))

(fn `UserConstructionScript`)